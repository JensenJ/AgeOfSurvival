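; BPEnvironment applies lighting and sky settings to the level's Sun and SkySphere through a single Environment function.
; It rotates the Sun, updates the sky's sun direction, copies brightness, cloud, star and color values, then refreshes the sky material.
; Weather is only printed as debug text, while Season, Temp, WindStrength and WindAngle are accepted but unused.
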(fn `Environment`
  (params (SunAngle :type "Rotator Structure") (Season :type "ESeasonEnum Enum" :default "ENone") (Temp :type String) (WindStrength :type String) (WindAngle :type String) (SunBrightness :type "Float (double-precision)") (CloudSpeed :type "Float (double-precision)") (CloudOpacity :type "Float (double-precision)") (StarOpacity :type "Float (double-precision)") (Weather :type "EWeatherEnum Enum" :default "ENone") (ZenithColor :type "LinearColor Structure") (HorizonColor :type "LinearColor Structure") (CloudColor :type "LinearColor Structure") (OverallColor :type "LinearColor Structure"))
  (bind _skysphere (`self.SkySphere`))
  (`self.K2_SetActorRotation` (`self.Sun`) SunAngle false)
  (`|ExecutionSequence`
    (:`then_0`
      (`/Engine/EngineSky/BP_Sky_Sphere.UpdateSunDirection` _skysphere)
      (set `/Engine/EngineSky/BP_Sky_Sphere.Sun brightness` SunBrightness _skysphere)
      (set `/Engine/EngineSky/BP_Sky_Sphere.Cloud speed` CloudSpeed _skysphere)
      (set `/Engine/EngineSky/BP_Sky_Sphere.Cloud opacity` CloudOpacity _skysphere)
      (set `/Engine/EngineSky/BP_Sky_Sphere.Stars brightness` StarOpacity _skysphere))
    (:`then_1`
      (set `/Engine/EngineSky/BP_Sky_Sphere.Zenith Color` ZenithColor _skysphere)
      (set `/Engine/EngineSky/BP_Sky_Sphere.Horizon color` HorizonColor _skysphere)
      (set `/Engine/EngineSky/BP_Sky_Sphere.Cloud color` CloudColor _skysphere)
      (set `/Engine/EngineSky/BP_Sky_Sphere.Overall Color` OverallColor _skysphere))
    (:`then_2`
      (`/Engine/EngineSky/BP_Sky_Sphere.RefreshMaterial` _skysphere)
      (`KismetSystemLibrary.PrintString` (`|GetEnumeratorNameAsString` Weather)))))

(fn `UserConstructionScript`)