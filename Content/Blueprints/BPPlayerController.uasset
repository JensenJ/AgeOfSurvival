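; Player controller Blueprint that opens and closes the inventory screen and lets it be refreshed.
; The ToggleInventory input creates the Inventory widget on first use, then shows or removes it from the viewport, disabling the player character's CanMove while it is open.
; A ReloadInventory event tells the existing widget to reload its items.
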(event `self.ReloadInventory`
  (bind _inventorywidget (`self.InventoryWidget`))
  (`/Engine/EditorBlueprintResources/StandardMacros.IsValid` _inventorywidget
    (:`Is Valid`
      (bind _asinventory (cast `/Game/UI/Inventory` _inventorywidget))
      (`/Game/UI/Inventory.LoadInventoryItems` _asinventory))))

(event `InputAction|ToggleInventory`
  (params (Key :type "Key Structure"))
  (bind _inventorywidget (`self.InventoryWidget`))
  (:`Pressed`
    (bind _ascppcharacter_player (cast `CPPCharacterPlayer` (`GameplayStatics.GetPlayerCharacter` 0)))
    (if (`Widget.IsVisible` _inventorywidget)
      (`Widget.RemoveFromParent` _inventorywidget)
      (set `CPPCharacterPlayer.bCanMove` true _ascppcharacter_player)
      (else
        (set `CPPCharacterPlayer.bCanMove` false _ascppcharacter_player)
        (`/Engine/EditorBlueprintResources/StandardMacros.IsValid` _inventorywidget
          (:`Is Valid`
            _)
          (:`Is Not Valid`
            (bind _returnvalue (`|CreateWidget` "/Game/UI/Inventory.Inventory_C"))
            (bind _output_get (set `self.InventoryWidget` _returnvalue))))
        (`UserWidget.AddToViewport` _output_get 0)))))

(fn `UserConstructionScript`)