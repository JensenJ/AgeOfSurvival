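; Player character Blueprint that drives animation state and supports switching between first-person and third-person views.
; Each Tick, it casts the mesh's anim instance to ABP_Character and copies walking and crouching flags, deriving IsMoving from forward and right movement input.
; The walking and crouching flags are also printed every frame as debug output.
; SwitchPOV activates one of the two cameras and deactivates the other based on a boolean.
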(event `self.ReceiveTick`
  (params (DeltaSeconds :type "Float (single-precision)"))
  (bind _asabp_character (cast `/Game/Animations/ABP_Character` (`SkeletalMeshComponent.GetAnimInstance` (`self.Mesh`))))
  (if (or (!= (`self.GetInputAxisValue`) 0.0) (!= (`self.GetInputAxisValue`) 0.0))
    (set `/Game/Animations/ABP_Character.IsMoving` true _asabp_character)
    (else
      (set `/Game/Animations/ABP_Character.IsMoving` false _asabp_character)))
  (if (`self.bIsWalking`)
    (set `/Game/Animations/ABP_Character.IsWalking` true _asabp_character)
    (else
      (set `/Game/Animations/ABP_Character.IsWalking` false _asabp_character)))
  (if (`self.bIsCrouching`)
    (set `/Game/Animations/ABP_Character.IsCrouching` true _asabp_character)
    (else
      (set `/Game/Animations/ABP_Character.IsCrouching` false _asabp_character)))
  (`KismetSystemLibrary.PrintString` (`KismetStringLibrary.Conv_BoolToString` (`self.bIsWalking`)))
  (`KismetSystemLibrary.PrintString` (`KismetStringLibrary.Conv_BoolToString` (`self.bIsCrouching`))))

(event `self.SwitchPOV`
  (params (bIsFirstPerson :type Boolean))
  (bind _firstpersoncamera (`self.FirstPersonCamera`))
  (bind _thirdpersoncamera (`self.ThirdPersonCamera`))
  (if bIsFirstPerson
    (`ActorComponent.Activate` _firstpersoncamera true)
    (`ActorComponent.Deactivate` _thirdpersoncamera)
    (else
      (`ActorComponent.Deactivate` _firstpersoncamera)
      (`ActorComponent.Activate` _thirdpersoncamera true))))

(fn `UserConstructionScript`)